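; Player hero Blueprint that handles pausing, the quest UI, coin counting and slot-based save/load.
; BeginPlay creates the Narrative quest UI and a hidden PauseMenu; P pauses and reveals the menu, while Q pauses and opens the quest journal.
; Saving writes player transform, coin count and BP_Coin transforms to CharacterSave.
; Loading restores them asynchronously, matching coins by GetAllActorsOfClass array index.
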(event `Key|P`
  (params (Key :type "Key Structure"))
  (bind _returnvalue (`GameplayStatics.GetPlayerController` 0))
  (bind _paused (`self.Paused`))
  ;[1 1 1] Pause Game
  (:`Pressed`
    (`GameplayStatics.SetGamePaused` true)
    (`Widget.SetVisibility` (`self.Paused`) "Visible")
    (set `PlayerController.bShowMouseCursor` true _returnvalue)
    (`Widget.SetIsEnabled` _paused true)
    (`WidgetBlueprintLibrary.SetInputMode_UIOnlyEx` _returnvalue _paused "LockAlways")))

(event `CustomEvent`
  (bind _returnvalue (`GameplayStatics.GetPlayerController` 0))
  ;[1 1 1] Pause Game
  (bind _returnvalue_2 (`|CreateWidget` "/Game/Saving/InGameMenu/PauseMenu.PauseMenu_C"))
  (bind _output_get (set `self.Paused` _returnvalue_2))
  (`Widget.SetVisibility` _output_get "Hidden")
  (`UserWidget.AddToViewport` _output_get 0)
  (`WidgetBlueprintLibrary.SetInputMode_GameOnly` _returnvalue)
  (set `PlayerController.bShowMouseCursor` false _returnvalue))

(event `Saving`
  (params (FileName :type String))
  ;[1 1 1] Saving System
  (bind _returnvalue (`GameplayStatics.DoesSaveGameExist` FileName))
  (if _returnvalue
    (bind _returnvalue_2 (`GameplayStatics.LoadGameFromSlot` FileName))
    (bind _ascharacter_save (cast `/Game/Saving/CharacterSave` _returnvalue_2))
    (set `/Game/Saving/CharacterSave.CharacterPosition` (`self.GetTransform` (`GameplayStatics.GetPlayerCharacter` 0)) _ascharacter_save)
    (bind _outactors (`GameplayStatics.GetAllActorsOfClass` "/Game/Saving/Coins/BP_Coin.BP_Coin_C"))
    (`KismetArrayLibrary.Array_Clear` (`self.CurrentCoinPositions`))
    (for _array_element _outactors
      (`KismetArrayLibrary.Array_Add` (`self.CurrentCoinPositions`) (`self.GetTransform` _array_element)))
    (set `/Game/Saving/CharacterSave.CoinPositions` (`self.CurrentCoinPositions`) _ascharacter_save)
    (set `/Game/Saving/CharacterSave.CoinCount` (`self.CoinCount`) _ascharacter_save)
    (`GameplayStatics.SaveGameToSlot` _ascharacter_save FileName)
    (else
      (bind _returnvalue_3 (`GameplayStatics.CreateSaveGameObject` "/Game/Saving/CharacterSave.CharacterSave_C"))
      (bind _output_get (set `self.SaveGame1` _returnvalue_3))
      (set `/Game/Saving/CharacterSave.CharacterPosition` (`self.GetTransform` (`GameplayStatics.GetPlayerCharacter` 0)) _output_get)
      (bind _outactors_2 (`GameplayStatics.GetAllActorsOfClass` "/Game/Saving/Coins/BP_Coin.BP_Coin_C"))
      (`KismetArrayLibrary.Array_Clear` (`self.CurrentCoinPositions`))
      (for _array_element_2 _outactors_2
        (`KismetArrayLibrary.Array_Add` (`self.CurrentCoinPositions`) (`self.GetTransform` _array_element_2)))
      (set `/Game/Saving/CharacterSave.CoinPositions` (`self.CurrentCoinPositions`) _output_get)
      (set `/Game/Saving/CharacterSave.CoinCount` (`self.CoinCount`) _output_get)
      (`GameplayStatics.SaveGameToSlot` _output_get FileName))))

(event `IncreaseCoinCount`
  ;[1 1 1] Saving System
  (set `self.CoinCount` (+ (`self.CoinCount`) 1)))

(event `Loading`
  (params (FileName :type String))
  ;[1 1 1] Saving System
  (bind _returnvalue (`GameplayStatics.DoesSaveGameExist` FileName))
  (if _returnvalue
    (bind _savegame (`AsyncActionHandleSaveGame.AsyncLoadGameFromSlot` FileName)
      (:`Completed`
        (bind _ascharacter_save (cast `/Game/Saving/CharacterSave` _savegame)
          (:`then`
            (`self.K2_SetActorTransform` (`GameplayStatics.GetPlayerCharacter` 0) (`/Game/Saving/CharacterSave.CharacterPosition` _ascharacter_save) false false)
            (bind _output_get (set `self.CurrentCoinPositions` (`/Game/Saving/CharacterSave.CoinPositions` _ascharacter_save)))
            (bind _outactors (`GameplayStatics.GetAllActorsOfClass` "/Game/Saving/Coins/BP_Coin.BP_Coin_C"))
            (for (_array_element _array_index) _outactors
              (`self.K2_SetActorTransform` _array_element (`|GetArrayItem` _output_get _array_index) false false))
            (set `self.CoinCount` (`/Game/Saving/CharacterSave.CoinCount` _ascharacter_save)))
          (:`CastFailed`
            (`KismetSystemLibrary.PrintString` "Cast Save Failed" true true (struct :`G` 0.66 :`B` 1.0 :`A` 1.0) 10.0)))))
    (else
      (`KismetSystemLibrary.PrintString` "Doesn't Exist" true true (struct :`G` 0.66 :`B` 1.0 :`A` 1.0) 10.0))))

(event `self.ReceiveBeginPlay`
  (bind _returnvalue (`GameplayStatics.GetPlayerController` 0))
  ;[1 1 1] Quests
  (bind _returnvalue_2 (`|CreateWidget` "/Game/Narrative/UI_Narrative/BP_NarrativeDefaultUI.BP_NarrativeDefaultUI_C" null (`self.Narrative`)))
  (`UserWidget.AddToViewport` _returnvalue_2 0)
  (bind _returnvalue_3 (`|CreateWidget` "/Game/Saving/InGameMenu/PauseMenu.PauseMenu_C"))
  (bind _output_get (set `self.Paused` _returnvalue_3))
  (`Widget.SetVisibility` _output_get "Hidden")
  (`UserWidget.AddToViewport` _output_get 0)
  (`WidgetBlueprintLibrary.SetInputMode_GameOnly` _returnvalue)
  (set `PlayerController.bShowMouseCursor` false _returnvalue))

(event `Key|Q`
  (params (Key :type "Key Structure"))
  ;[1 1 1] Quests
  (:`Pressed`
    (`GameplayStatics.SetGamePaused` true)
    (bind _returnvalue (`|CreateWidget` "/Narrative/NarrativeUI/Widgets/BP_QuestJournal.BP_QuestJournal_C" null (`self.Narrative`)))
    (`UserWidget.AddToViewport` _returnvalue 0)))

(event `self.ResetGame`
  (`self.Die`))

(fn `UserConstructionScript`)