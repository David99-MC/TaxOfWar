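; BP_Menu3D is a menu actor in the world that hands the player's view to linked menu actors.
; On BeginPlay it binds to its Menu3DWidget's transition event, which supplies an index into the LinkedMenus array.
; A valid index moves collision from this menu to the target, then eases the player's view target over to it with a timed camera blend.
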(event `self.ReceiveBeginPlay`
  (bind _asmenu_3dwidget (cast `/Game/3D_Menu/Widgets/Menu3DWidget` (`WidgetComponent.GetUserWidgetObject` (`self.Widget`))))
  (add `/Game/3D_Menu/Widgets/Menu3DWidget.TransitionToLinkedMenu` _asmenu_3dwidget (delegate `OnTransition`)))

(event `OnTransition`
  (params (MenuIndex :type Integer))
  (if (`KismetArrayLibrary.Array_IsValidIndex` (`self.LinkedMenus`) MenuIndex)
    (`self.TransitionTo` (`|GetArrayItem` (`self.LinkedMenus`) MenuIndex))))

(event `TransitionTo`
  (params (`New Menu` :type "/Game/3D_Menu/BP_Menu3D Object Reference"))
  (`self.SetActorEnableCollision` false)
  (`self.SetActorEnableCollision` `New Menu` true)
  (`PlayerController.SetViewTargetWithBlend` (`GameplayStatics.GetPlayerController` 0) `New Menu` 2.0 "VTBlend_EaseInOut" 1.0 false))

(fn `UserConstructionScript`)